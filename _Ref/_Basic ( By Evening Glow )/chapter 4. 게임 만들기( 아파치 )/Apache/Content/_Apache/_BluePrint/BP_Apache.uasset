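; Player-controlled Apache helicopter that flies, turns, fires paired rockets with muzzle effects and prints its count of destroyed anti-aircraft guns.
; Keyed movement and yaw axes are eased through MyLinearInterp (FInterpTo), then applied as local offsets and rotation.
; Turning also banks the SpringArm within clamped roll, while mouse and experimental touch drag drive its pitch via ScrollUpDown.
; Rotor animation and arm yaw scrolling are left unconnected.
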(event `InputAxis|apache forward/back`
  (params (AxisValue :type "Float (single-precision)")))

(event `InputAxis|apache forward/back`
  (params (AxisValue :type "Float (single-precision)"))
  (bind _return_value (`self.MyLinearInterp` AxisValue (`self.currentX`) (`self.SpeedMove`)))
  (set `self.currentX` _return_value)
  (`self.K2_AddActorLocalOffset` (`KismetMathLibrary.MakeVector` _return_value) true))

(event `InputAxis|apache left/right`
  (params (AxisValue :type "Float (single-precision)"))
  (bind _return_value (`self.MyLinearInterp` AxisValue (`self.currentY`) (`self.SpeedMove`)))
  (set `self.currentY` _return_value)
  (`self.K2_AddActorLocalOffset` (`KismetMathLibrary.MakeVector` 0.0 _return_value) true))

(event `self.ReceiveTick`
  (params (DeltaSeconds :type "Float (single-precision)"))
  (`|ExecutionSequence`
    (:`then_0`
      ;[1 1 1] 터치 관련 R&D 필요
      (bind (_move_x _move_y) (`self.TouchMove`))
      (if (`self.IsMoved`)
        (`self.ScrollUpDown` _move_y)))
    (:`then_1`
      ;[1 1 1] 파괴한 대공포 갯수 출력.
      (`KismetSystemLibrary.Delay` 0.2)
      (`KismetSystemLibrary.PrintString` (`KismetStringLibrary.Conv_IntToString` (`self.KillCount`))))))

(event `InputAxis|apache up/down`
  (params (AxisValue :type "Float (single-precision)"))
  (bind _return_value (`self.MyLinearInterp` AxisValue (`self.currentZ`) (`self.SpeedMove`)))
  (set `self.currentZ` _return_value)
  (`self.K2_AddActorLocalOffset` (`KismetMathLibrary.MakeVector` 0.0 0.0 _return_value) true))

(event `InputAxis|apache rotate`
  (params (AxisValue :type "Float (single-precision)"))
  (bind _armroll (`self.armRoll`))
  (bind _return_value (`self.MyLinearInterp` AxisValue (`self.currentYaw`) (`self.SpeedRot`)))
  (set `self.currentYaw` _return_value)
  (`self.K2_AddActorLocalRotation` (`KismetMathLibrary.MakeRotator` 0.0 0.0 _return_value))
  (bind _return_value_2 (`self.MyLinearInterp` AxisValue _armroll -1500.0))
  (set `self.armRoll` (`KismetMathLibrary.FClamp` _return_value_2 -15.0 15.0))
  (`SceneComponent.K2_SetWorldRotation` (`self.SpringArm`) (`KismetMathLibrary.MakeRotator` _armroll (`self.armPitch`) (+ (.yaw (`self.K2_GetActorRotation`)) (`self.armYaw`))) false false))

(event `InputAction|mobile touch`
  (params (Key :type "Key Structure"))
  ;[1 1 1] 터치 관련 R&D 필요
  (:`Pressed`
    (`self.TouchStart`))
  (:`Released`
    (set `self.IsMoved` false)))

(event `InputAxis|mouse rotate LR`
  (params (AxisValue :type "Float (single-precision)"))
  (bind _returnvalue (`KismetMathLibrary.FClamp` (- (`self.armRoll`) AxisValue) -25.0 25.0))
  ;[1 1 1] 헬기 동체 회전
  (`self.K2_AddActorLocalRotation` (`KismetMathLibrary.MakeRotator` 0.0 0.0 AxisValue))
  ;[1 1 1] 스프링 암 회전
  (set `self.armRoll` _returnvalue)
  (`SceneComponent.K2_SetWorldRotation` (`self.SpringArm`) (`KismetMathLibrary.MakeRotator` _returnvalue (`self.armPitch`) (+ (.yaw (`self.K2_GetActorRotation`)) (`self.armYaw`))) false false))

(event `InputAction|apache Shoot`
  (params (Key :type "Key Structure"))
  (bind _returnvalue (`SceneComponent.K2_GetComponentToWorld` (`self.SpawnRight`)))
  (bind _returnvalue_2 (`SceneComponent.K2_GetComponentToWorld` (`self.SpawnLeft`)))
  (:`Pressed`
    (`|ExecutionSequence`
      (:`then_0`
        (`|SpawnActorFromClass` "/Game/_Apache/_BluePrint/BP_Rocket.BP_Rocket_C" _returnvalue "Undefined" "OverrideRootScale" null null)
        (`GameplayStatics.SpawnEmitterAtLocation` "/Game/_Apache/_Particle/P_Explosion2.P_Explosion2" (`KismetMathLibrary.TransformLocation` _returnvalue)))
      (:`then_1`
        (`|SpawnActorFromClass` "/Game/_Apache/_BluePrint/BP_Rocket.BP_Rocket_C" _returnvalue_2 "Undefined" "OverrideRootScale" null null)
        (`GameplayStatics.SpawnEmitterAtLocation` "/Game/_Apache/_Particle/P_Explosion2.P_Explosion2" (`KismetMathLibrary.TransformLocation` _returnvalue_2))))))

(event `InputAxis|mouse rotate TB`
  (params (AxisValue :type "Float (single-precision)"))
  (`self.ScrollUpDown` AxisValue) ; 스프링 암 pitch 회전
)

(fn `GetTouchPos`
  (returns (x :type "Float (double-precision)") (y :type "Float (double-precision)") (`Is Moved` :type Boolean))
  (bind (_locationx _locationy _biscurrentlypressed) (`PlayerController.GetInputTouchState` (`GameplayStatics.GetPlayerController` 0) "Touch1"))
  (return _locationx _locationy _biscurrentlypressed))

(fn `MyLinearInterp`
  (params (`Axis Value` :type "Float (double-precision)") (`Current Value` :type "Float (double-precision)") (Speed :type "Float (double-precision)"))
  (returns (`Return Value` :type "Float (double-precision)"))
  (bind _returnvalue (`GameplayStatics.GetWorldDeltaSeconds`))
  (return (`KismetMathLibrary.FInterpTo` `Current Value` (* `Axis Value` Speed _returnvalue) _returnvalue 6.0)))

(fn `ScrollLeftRight`
  (params (`Axis Value` :type "Float (double-precision)"))
  (bind _armyaw (`self.armYaw`))
  (set `self.armYaw` (`KismetMathLibrary.FClamp` (+ `Axis Value` _armyaw) -80.0 80.0))
  (`SceneComponent.K2_SetWorldRotation` (`self.SpringArm`) (`KismetMathLibrary.MakeRotator` (`self.armPitch`) (`self.armRoll`) (+ _armyaw (.yaw (`self.K2_GetActorRotation`)))) false false))

(fn `ScrollUpDown`
  (params (`Axis Value` :type "Float (double-precision)"))
  (bind _returnvalue (`KismetMathLibrary.FClamp` (+ `Axis Value` (`self.armPitch`)) -80.0 30.0))
  (set `self.armPitch` _returnvalue)
  (`SceneComponent.K2_SetWorldRotation` (`self.SpringArm`) (`KismetMathLibrary.MakeRotator` (`self.armRoll`) _returnvalue (+ (.yaw (`self.K2_GetActorRotation`)) (`self.armYaw`))) false false))

(fn `TouchMove`
  (returns (`Move X` :type "Float (double-precision)") (`Move Y` :type "Float (double-precision)"))
  (bind (_x _y _is_moved) (`self.GetTouchPos`))
  (set `self.IsMoved` _is_moved)
  (return (`KismetMathLibrary.FClamp` (- _x (`self.touchX`)) -1.0) (`KismetMathLibrary.FClamp` (- _y (`self.touchY`)) -1.0)))

(fn `TouchStart`
  (bind (_x _y _is_moved) (`self.GetTouchPos`))
  (set `self.touchX` _x)
  (set `self.touchY` _y)
  (set `self.IsMoved` _is_moved))

(fn `UserConstructionScript`)