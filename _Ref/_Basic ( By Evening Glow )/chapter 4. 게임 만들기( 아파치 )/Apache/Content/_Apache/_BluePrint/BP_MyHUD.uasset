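; BP_MyHUD is a HUD Blueprint that draws a simple BlueRect material square near the top-left of the screen through DrawHUD.
; Helper functions store the screen size and draw horizontally centered text, using the measured pixel width of the string to find its X position.
; The nodes that set the screen size, draw the centered test string and print debug text are disconnected, so only the square renders.
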(event `self.ReceiveDrawHUD`
  (params (SizeX :type Integer) (SizeY :type Integer))
  (`self.DrawMaterialSimple` "/Game/_Apache/_Material/BlueRect.BlueRect" 50.0 50.0 200.0 200.0) ; 간단한 머터리얼 출력
)

(fn `DrawTextCenter`
  (params (Text :type String) (Color :type "LinearColor Structure") (ScreenY :type "Float (double-precision)") (Font :type "Font Object Reference") (Scale :type "Float (double-precision)"))
  (bind _return_value (`self.GetCenterPos` (`self.GetTextSize` Text Font Scale))) ; 출력위치를 계산( 단, 너비만 적용)
  (`self.DrawText` Text Color _return_value ScreenY Font Scale))

(fn `GetCenterPos`
  (params (width :type "Float (double-precision)"))
  (returns (`Return Value` :type "Float (double-precision)"))
  (return (/ (- (`self.ScreenWidth`) width) 2.0)))

(fn `SetScreenSize`
  (params (width :type Integer) (height :type Integer))
  (set `self.ScreenWidth` (`KismetMathLibrary.Conv_IntToDouble` width))
  (set `self.ScreenHeight` (`KismetMathLibrary.Conv_IntToDouble` height)))

(fn `UserConstructionScript`)