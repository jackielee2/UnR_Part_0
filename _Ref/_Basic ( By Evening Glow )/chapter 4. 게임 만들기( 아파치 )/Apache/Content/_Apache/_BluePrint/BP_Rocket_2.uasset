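; BP_Rocket_2 is a rocket projectile actor that explodes when its Tirgger component hits something.
; The hit event, gated by DoOnce, spawns an explosion particle and calls play-sound at the rocket's location, with no sound asset shown on that call.
; A short delay before destroying the actor lets the struck object register the hit.
; Two alternative explosion approaches, immediate destruction and component-only destruction, remain unconnected.
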(event `self.Tirgger.OnComponentHit`
  (params (HitComponent :type "PrimitiveComponent Object Reference") (OtherActor :type "Actor Object Reference") (OtherComp :type "PrimitiveComponent Object Reference") (NormalImpulse :type "Vector Structure") (Hit :type "HitResult Structure (by ref)"))
  (bind _returnvalue (`self.K2_GetActorLocation`))
  ;[1 1 1] 로켓에 충돌한 오브젝트가 충돌 이벤트를 인지 할 수 있도록 시간 지연 적용.
  (`/Engine/EditorBlueprintResources/StandardMacros.DoOnce` false
    (:`Completed`
      (`GameplayStatics.SpawnEmitterAtLocation` "/Game/_Apache/_Particle/P_Explosion3.P_Explosion3" _returnvalue (struct) (1.0 1.0 1.0) false)
      (`GameplayStatics.PlaySoundAtLocation` null _returnvalue (struct) 1.0 1.0 0.0 null null null)
      (`KismetSystemLibrary.Delay` 0.1)
      (`self.K2_DestroyActor`))))

(fn `UserConstructionScript`)