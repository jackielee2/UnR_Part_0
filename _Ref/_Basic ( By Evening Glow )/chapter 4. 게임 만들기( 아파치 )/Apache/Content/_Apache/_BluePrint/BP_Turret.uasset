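; Anti-aircraft turret truck that tracks the player's helicopter and fires rocket pairs at it.
; Tick computes look-at rotation and distance, turns the gun with clamped pitch within search range, and fires from both muzzles within fire range on a delayed cooldown.
; The construction script randomizes each muzzle's relative yaw in opposite directions.
; The first hit on the truck disables it, increments BP_Apache's kill count, and removes it after a delay.
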(event `self.ReceiveTick`
  (params (DeltaSeconds :type "Float (single-precision)"))
  ;[1 1 1] 포탑 방향/거리 연산, 포탑 회전, 로켓 발사 ( 커스텀 이벤트 적용 후 )
  (if (not (`self.isDestroyed`))
    (`self.CE_CalcuateRotDist`)
    (`self.CE_RotateTurret`)
    (if (<= (`self.targetDist`) (`self.fireRange`))
      (`self.CE_ShotRocket`))))

(event `CE_ShotRocket`
  (bind _returnvalue (`SceneComponent.K2_GetComponentToWorld` (`self.SpawnRight`)))
  (bind _returnvalue_2 (`SceneComponent.K2_GetComponentToWorld` (`self.SpawnLeft`)))
  ;[1 1 1] 대공포가 일정시간마다 로켓을 발사하는 커스텀 이벤트
  (if (`self.canFire`)
    (set `self.canFire` false)
    (`|SpawnActorFromClass` "/Game/_Apache/_BluePrint/BP_Rocket_2.BP_Rocket_2_C" _returnvalue "Undefined" "OverrideRootScale" null null)
    (`GameplayStatics.SpawnEmitterAtLocation` "/Game/_Apache/_Particle/P_Explosion2.P_Explosion2" (`KismetMathLibrary.TransformLocation` _returnvalue))
    (`|SpawnActorFromClass` "/Game/_Apache/_BluePrint/BP_Rocket_2.BP_Rocket_2_C" _returnvalue_2 "Undefined" "OverrideRootScale" null null)
    (`GameplayStatics.SpawnEmitterAtLocation` "/Game/_Apache/_Particle/P_Explosion2.P_Explosion2" (`KismetMathLibrary.TransformLocation` _returnvalue_2))
    (`KismetSystemLibrary.Delay` (`self.delayTime`)) ; 지정 시간동안 실행 지연.
    (set `self.canFire` true)))

(event `CE_CalcuateRotDist`
  (bind _returnvalue (`GameplayStatics.GetPlayerPawn` 0))
  ;[1 1 1] 대공포와 헬기의 거리와 방향을 연산하는 커스텀 이벤트
  (set `self.targetRotation` (`KismetMathLibrary.FindLookAtRotation` (`self.K2_GetActorLocation`) (`self.K2_GetActorLocation` _returnvalue)))
  (set `self.targetDist` (`self.GetDistanceTo` _returnvalue)))

(event `CE_RotateTurret`
  ;[1 1 1] 대공포 회전
  (if (<= (`self.targetDist`) (`self.searchRange`))
    (`SceneComponent.K2_SetWorldRotation` (`self.9_Turret_Gun_DM`) (`KismetMathLibrary.MakeRotator` 0.0 (`KismetMathLibrary.FClamp` (.pitch (`self.targetRotation`)) 0.0 40.0) (.yaw (`self.targetRotation`))) false false)))

(event `self.9_Turret_Truck_DM.OnComponentHit`
  (params (HitComponent :type "PrimitiveComponent Object Reference") (OtherActor :type "Actor Object Reference") (OtherComp :type "PrimitiveComponent Object Reference") (NormalImpulse :type "Vector Structure") (Hit :type "HitResult Structure (by ref)"))
  ;[1 1 1] 파괴된 대공포의 로켓 발사 막기.
  (`/Engine/EditorBlueprintResources/StandardMacros.DoOnce` false
    (:`Completed`
      (set `self.isDestroyed` true)
      (`self.SetKillCount`) ; 파괴된 대공포의 수 증가
      ;[1 1 1] 파괴된 대공포 잔해 제거
      (`KismetSystemLibrary.Delay` 3.0)
      (`self.K2_DestroyActor`))))

(fn `SetKillCount`
  (bind _asbp_apache (cast `/Game/_Apache/_BluePrint/BP_Apache` (`GameplayStatics.GetPlayerPawn` 0)))
  (set `/Game/_Apache/_BluePrint/BP_Apache.KillCount` (+ (`/Game/_Apache/_BluePrint/BP_Apache.KillCount` _asbp_apache) 1) _asbp_apache))

(fn `UserConstructionScript`
  (bind _returnvalue (`KismetMathLibrary.RandomFloatInRange` 0.5 1.2))
  (`SceneComponent.K2_SetRelativeRotation` (`self.SpawnLeft`) (`KismetMathLibrary.MakeRotator` 0.0 0.0 _returnvalue) false false) ; 씬의 대공포를 임의의 방향으로 회전시켜 배치할 수도 있으므로 절대좌표(Set World Rotation)을 사용하면 안된다.
  (`SceneComponent.K2_SetRelativeRotation` (`self.SpawnRight`) (`KismetMathLibrary.MakeRotator` 0.0 0.0 (* _returnvalue -1.0)) false false) ; 씬의 대공포를 임의의 방향으로 회전시켜 배치할 수도 있으므로 절대좌표(Set World Rotation)을 사용하면 안된다.
)